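; Gameplay ability for the player's umbrella attack, playing an attack montage on the owner's skeletal mesh.
; Each montage notify decrements the player's AttackQueue, letting the montage continue while queued attacks remain, as a combo chain.
; When the queue empties, it clears IsAttacking, blends the montage out and ends the ability.
; Montage completion, blend-out or interruption also clears IsAttacking and ends the ability.
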(event `self.K2_ActivateAbility`
  (`self.K2_CommitAbility`)
  (`|PlayMontage` (`.SkeletalMeshComponent` (break `GameplayAbilityActorInfo` (`self.GetActorInfo`))) "/Game/AnimationClips/ANIM_Attack.ANIM_Attack" 0.8
    (:`OnCompleted`
      (bind _asbp_player (cast `/Game/Blueprint/Player/BP_Player` (`.OwnerActor` (break `GameplayAbilityActorInfo` (`self.GetActorInfo`))) :!label _label))
      (set `/Game/Blueprint/Player/BP_Player.IsAttacking` false _asbp_player)
      (`self.K2_EndAbility`))
    (:`OnBlendOut`
      (goto _label))
    (:`OnInterrupted`
      (goto _label))
    (:`OnNotifyBegin`
      (bind _asbp_player_2 (cast `/Game/Blueprint/Player/BP_Player` (`.OwnerActor` (break `GameplayAbilityActorInfo` (`self.GetActorInfo`)))))
      (bind _result (`/Engine/EditorBlueprintResources/StandardMacros.DecrementInt` (`/Game/Blueprint/Player/BP_Player.AttackQueue` _asbp_player_2))
        (:`  `
          (if (not (> _result 0))
            (bind _asbp_player_3 (cast `/Game/Blueprint/Player/BP_Player` (`.OwnerActor` (break `GameplayAbilityActorInfo` (`self.GetActorInfo`)))))
            (set `/Game/Blueprint/Player/BP_Player.IsAttacking` false _asbp_player_3)
            (`AnimInstance.Montage_Stop` (`SkeletalMeshComponent.GetAnimInstance` (`.SkeletalMeshComponent` (break `GameplayAbilityActorInfo` (`self.GetActorInfo`)))) 0.45 "/Game/AnimationClips/ANIM_Attack.ANIM_Attack")
            (`self.K2_EndAbility`)))))))