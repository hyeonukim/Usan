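; Enemy AI character that detects the player, attacks in melee and takes damage.
; A vision sphere writes the player to the blackboard Target key on overlap and clears it on exit.
; ATK_01 turns toward its target and plays a random attack montage.
; DoDamage sphere-overlaps pawns at an arrow component, damaging those tagged Player, while incoming damage only lowers and prints Health, with no death handling.
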(event `self.SphereVision.OnComponentBeginOverlap`
  (params (OverlappedComponent :type "PrimitiveComponent Object Reference") (OtherActor :type "Actor Object Reference") (OtherComp :type "PrimitiveComponent Object Reference") (OtherBodyIndex :type Integer) (bFromSweep :type Boolean) (SweepResult :type "HitResult Structure (by ref)"))
  ;[0 0 0] Overlap Set, Get, and Clear Target
  (if true
    (bind _asbp_player (cast `/Game/Blueprint/Player/BP_Player` OtherActor))
    (`self.SetTarget` _asbp_player)))

(event `self.SphereVision.OnComponentEndOverlap`
  (params (OverlappedComponent :type "PrimitiveComponent Object Reference") (OtherActor :type "Actor Object Reference") (OtherComp :type "PrimitiveComponent Object Reference") (OtherBodyIndex :type Integer))
  ;[0 0 0] Overlap Set, Get, and Clear Target
  (if (== OtherActor (`self.GetTarget`))
    (`self.ClearTarget`)))

(event `ATK_01`
  (params (Target :type "Actor Object Reference"))
  (bind (_returnvalue_roll _returnvalue_pitch _returnvalue_yaw) (`KismetMathLibrary.BreakRotator` (`KismetMathLibrary.FindLookAtRotation` (`self.K2_GetActorLocation`) (`self.K2_GetActorLocation` Target))))
  ;[0 0 0] ATK_01
  (`|ExecutionSequence`
    (:`then_0`
      (`/Engine/EditorBlueprintResources/StandardMacros.IsValid` Target
        (:`Is Valid`
          (`KismetSystemLibrary.LogString` "Performing")
          (`self.K2_SetActorRotation` (`KismetMathLibrary.MakeRotator` 0.0 0.0 _returnvalue_yaw)))))
    (:`then_1`
      (`self.PlayAnimMontage` (`|GetArrayItem` (`self.AttackArray`) (`KismetMathLibrary.RandomIntegerInRange` 0 1))))))

(event `DoDamage`
  (bind _returnvalue (`SceneComponent.K2_GetComponentLocation` (`self.DamageArrow`)))
  ;[0 0 0] Do Damage
  (bind (_outactors _returnvalue_2) (`KismetSystemLibrary.SphereOverlapActors` _returnvalue (`self.DamageRadius`) (`|MakeArray` "ObjectTypeQuery3" :!type "EObjectTypeQuery Enum") null (`|MakeArray` self :!type "Actor Object Reference")))
  (`KismetSystemLibrary.DrawDebugSphere` _returnvalue 100.0 12 (struct :`R` 1.0 :`A` 1.0) 1.0 1.0)
  (if _returnvalue_2
    (for _array_element _outactors
      (if (`self.ActorHasTag` _array_element "Player")
        (`GameplayStatics.ApplyDamage` _array_element 0.2 (`self.GetController`) self)))))

(event `self.ReceiveAnyDamage`
  (params (Damage :type "Float (single-precision)") (DamageType :type "DamageType Object Reference") (InstigatedBy :type "Controller Object Reference") (DamageCauser :type "Actor Object Reference"))
  (bind _output_get (set `self.Health` (- (`self.Health`) Damage)))
  (`KismetSystemLibrary.PrintString` (`KismetStringLibrary.Concat_StrStr` "Health: " (`KismetStringLibrary.Conv_DoubleToString` _output_get))))

(fn `ClearTarget`
  (`BlackboardComponent.ClearValue` (`AIBlueprintHelperLibrary.GetBlackboard` (`AIBlueprintHelperLibrary.GetAIController` self)) "Target"))

(fn `GetTarget`
  (returns (Target :type "Actor Object Reference"))
  (return (cast `Actor` (`BlackboardComponent.GetValueAsObject` (`AIBlueprintHelperLibrary.GetBlackboard` (`AIBlueprintHelperLibrary.GetAIController` self)) "Target") :!pure true)))

(fn `SetTarget`
  (params (NewTarget :type "Actor Object Reference"))
  (`BlackboardComponent.SetValueAsObject` (`AIBlueprintHelperLibrary.GetBlackboard` (`AIBlueprintHelperLibrary.GetAIController` self)) "Target" NewTarget))

(fn `UserConstructionScript`)