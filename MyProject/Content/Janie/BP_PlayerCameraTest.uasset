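; Player character test Blueprint for a third-person-style camera with a toggleable target lock-on.
; Enhanced Input drives movement relative to control rotation, jumping, and look with optional per-axis inversion.
; The lock input flip-flops between storing the hit actor from a very large, debug-drawn Pawn sphere trace along the camera's forward and clearing it.
; Tick snaps control rotation toward any valid target.
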(event `self.ReceiveTick`
  (params (DeltaSeconds :type "Float (single-precision)"))
  (`self.HitTarget`
    (:`then`
      (`Controller.SetControlRotation` (`self.GetController`) (`KismetMathLibrary.FindLookAtRotation` (`self.K2_GetActorLocation`) (`self.K2_GetActorLocation` (`self.HitTarget`)))))
    (:`else`)))

(event `EnhancedInput|/Game/Inputs/Actions/INP_LockCamera`
  (params (ActionValue :type Boolean) (ElapsedSeconds :type "Float (double-precision)") (TriggeredSeconds :type "Float (double-precision)") (InputAction :type "InputAction Object Reference" :default "/Game/Inputs/Actions/INP_LockCamera.INP_LockCamera"))
  (bind _returnvalue (`self.K2_GetActorLocation`))
  (:`Triggered`
    (`/Engine/EditorBlueprintResources/StandardMacros.FlipFlop`
      (:`A`
        (bind _outhit (`KismetSystemLibrary.SphereTraceSingleForObjects` :`Start` _returnvalue :`End` (+ (* (`KismetMathLibrary.GetForwardVector` (`SceneComponent.K2_GetComponentRotation` (`self.Camera`))) 500.0) _returnvalue) :`Radius` 10000.0 :`ObjectTypes` (`|MakeArray` "ObjectTypeQuery3" :!type "EObjectTypeQuery Enum") :`DrawDebugType` "ForDuration"))
        (if true
          (set `self.HitTarget` (`.HitActor` (`GameplayStatics.BreakHitResult` _outhit)))))
      (:`B`
        (set `self.HitTarget` null)))))

(event `self.ReceiveBeginPlay`
  (bind _returnvalue (pcsubsystem `EnhancedInputLocalPlayerSubsystem` (`GameplayStatics.GetPlayerController` 0)))
  (`/Engine/EditorBlueprintResources/StandardMacros.IsValid` _returnvalue
    (:`Is Valid`
      (`EnhancedInputSubsystemInterface.AddMappingContext` _returnvalue "/Game/Inputs/IMC_Player.IMC_Player" 0 (struct)))))

(event `EnhancedInput|/Game/Inputs/Actions/INP_Jump`
  (params (ActionValue :type Boolean) (ElapsedSeconds :type "Float (double-precision)") (TriggeredSeconds :type "Float (double-precision)") (InputAction :type "InputAction Object Reference" :default "/Game/Inputs/Actions/INP_Jump.INP_Jump"))
  (:`Started`
    (`self.Jump`))
  (:`Completed`
    (`self.StopJumping`)))

(event `EnhancedInput|/Game/Inputs/Actions/INP_Move`
  (params (ActionValue :type "Vector2D Structure") (ElapsedSeconds :type "Float (double-precision)") (TriggeredSeconds :type "Float (double-precision)") (InputAction :type "InputAction Object Reference" :default "/Game/Inputs/Actions/INP_Move.INP_Move"))
  (bind (_returnvalue_roll _returnvalue_pitch _returnvalue_yaw) (`KismetMathLibrary.BreakRotator` (`self.GetControlRotation`)))
  (:`Triggered`
    (`self.AddMovementInput` (`KismetMathLibrary.GetRightVector` (`self.GetControlRotation`)) ActionValue_X)
    (`self.AddMovementInput` (`KismetMathLibrary.GetForwardVector` (`KismetMathLibrary.MakeRotator` _returnvalue_roll 0.0 _returnvalue_yaw)) ActionValue_Y)))

(event `EnhancedInput|/Game/Inputs/Actions/INP_Look`
  (params (ActionValue :type "Vector2D Structure") (ElapsedSeconds :type "Float (double-precision)") (TriggeredSeconds :type "Float (double-precision)") (InputAction :type "InputAction Object Reference" :default "/Game/Inputs/Actions/INP_Look.INP_Look"))
  (:`Triggered`
    (`self.AddControllerYawInput` (* ActionValue_X (`KismetMathLibrary.SelectFloat` -1.0 1.0 (`self.InvertCameraX`))))
    (`self.AddControllerPitchInput` (* ActionValue_Y (`KismetMathLibrary.SelectFloat` -1.0 1.0 (`self.InvertCameraY`))))))

(fn `UserConstructionScript`)